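; BP_AddCopyGun is a gun pickup actor that spins in place until collected.
; A looping timer set on BeginPlay rotates its skeletal mesh in small steps.
; EEvent, triggered from outside this graph, gives the first-person character its GunType, pushes TextMap to that character's TalkWidget, then destroys the pickup.
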(event Custom|Rotation
  (Transformation|AddLocalRotation (Variables|Default|GetSkeletalMesh) "0.000000,5.000000,0.000000" false false))

(event EventBeginPlay
  (bind _returnvalue (Actor|GetActorOfClass "/Game/FirstPerson/Blueprints/BP_FirstPersonCharacter.BP_FirstPersonCharacter_C"))
  (Variables|Default|SetPlayer _returnvalue)
  (Utilities|Time|SetTimerbyFunctionName 0 "Rotation" 0.01 true))

(event Collision|EventActorBeginOverlap
  (params (OtherActor :type Actor%20Object%20Reference)))

(event EventEEvent
  (bind _returnvalue (Actor|GetActorOfClass "/Game/FirstPerson/Blueprints/BP_FirstPersonCharacter.BP_FirstPersonCharacter_C"))
  (Default|AddGunType _returnvalue (Variables|Default|GetGunType))
  (Default|AddText (Variables|/Game/FirstPerson/Blueprints/BP_FirstPersonCharacter.BP_FirstPersonCharacter_C|GetTalkWidget _returnvalue) (Variables|Default|GetText%20Map))
  (Actor|DestroyActor))

(fn ConstructionScript)