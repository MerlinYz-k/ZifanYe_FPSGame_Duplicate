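; BP_AutoDoor is an automatic door that slides its Cube between its starting location and ChangeLoc using timeline-driven lerps.
; Doors flagged First open on BeginPlay, turning Cube1 and level meshes named LightGreen red.
; Other doors open when BP_FirstPersonCharacter enters Box, which disables its collision and plays a sound regardless of the flag.
; Custom events Reverse (green indicator, backward move) and LastMove (sound, forward move) use separate timelines.
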(event OnComponentBeginOverlap(Box)
  (params (OverlappedComponent :type Primitive%20Component%20Object%20Reference) (OtherActor :type Actor%20Object%20Reference) (OtherComp :type Primitive%20Component%20Object%20Reference) (OtherBodyIndex :type Integer) (bFromSweep :type Boolean) (SweepResult :type Hit%20Result%20Structure%20%28by%20ref%29))
  (Utilities|Casting|CastToBP_FirstPersonCharacter OtherActor)
  (Collision|SetCollisionEnabled (Variables|Default|GetBox) "NoCollision")
  (Audio|PlaySound2D "/Game/sound/E5高科技自动门-自动门开门机械声-科技感短视频转场_爱给网_aigei_com.E5高科技自动门-自动门开门机械声-科技感短视频转场_爱给网_aigei_com" 1.0 1.0 0.0 0 0)
  (if (not (Variables|Default|GetFirst))
    (bind _newtrack_0 (Timeline|Timeline PlayFromStart)
      (:Update
        (Transformation|SetWorldLocation (Variables|Default|GetCube) (Math|Vector|Lerp(Vector) (Variables|Default|GetLoc) (Variables|Default|GetchangeLoc) _newtrack_0) false false)))))

(event Custom|Reverse
  (Rendering|Material|SetMaterial (Variables|Default|GetCube1) 0 "/Game/GreenBasicShapeMaterial.GreenBasicShapeMaterial")
  (bind _newtrack_0 (Timeline|Timeline_0 ReverseFromEnd)
    (:Update
      (Transformation|SetWorldLocation (Variables|Default|GetCube) (Math|Vector|Lerp(Vector) (Variables|Default|GetLoc) (Variables|Default|GetchangeLoc) _newtrack_0) false false))))

(event Custom|LastMove
  (Audio|PlaySound2D "/Game/sound/E5高科技自动门-自动门开门机械声-科技感短视频转场_爱给网_aigei_com.E5高科技自动门-自动门开门机械声-科技感短视频转场_爱给网_aigei_com" 1.0 1.0 0.0 0 0)
  (bind _newtrack_0 (Timeline|Timeline_1 PlayFromStart)
    (:Update
      (Transformation|SetWorldLocation (Variables|Default|GetCube) (Math|Vector|Lerp(Vector) (Variables|Default|GetLoc) (Variables|Default|GetchangeLoc) _newtrack_0) false false))))

(event EventBeginPlay
  (Variables|Default|SetLoc (Transformation|GetWorldLocation (Variables|Default|GetCube)))
  (if (Variables|Default|GetFirst)
    (Rendering|Material|SetMaterial (Variables|Default|GetCube1) 0 "/Game/RedBasicShapeMaterial1.RedBasicShapeMaterial1")
    (bind _outactors (Actor|GetAllActorsOfClass "/Script/Engine.StaticMeshActor"))
    (for _array_element _outactors
      (if (Utilities|Enum|Equal(Enum) (Utilities|GetDisplayName _array_element) "LightGreen")
        (Rendering|Material|SetMaterial (Variables|/Script/Engine.StaticMeshActor|GetStaticMeshComponent _array_element) 0 "/Game/RedBasicShapeMaterial1.RedBasicShapeMaterial1")))
    (bind _newtrack_0 (Timeline|Timeline PlayFromStart)
      (:Update
        (Transformation|SetWorldLocation (Variables|Default|GetCube) (Math|Vector|Lerp(Vector) (Variables|Default|GetLoc) (Variables|Default|GetchangeLoc) _newtrack_0) false false)))))

(event Collision|EventActorBeginOverlap
  (params (OtherActor :type Actor%20Object%20Reference)))

(event EventTick
  (params (DeltaSeconds :type Float%20%28single-precision%29)))

(fn ConstructionScript)