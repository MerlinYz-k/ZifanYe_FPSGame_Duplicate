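; BP_Box is a physics box that the first-person character can push, grab and release.
; AddForce applies a velocity-change impulse to the Cube along a given direction, scaled by Power.
; Traction grabs the Cube with the character's PhysicsHandle and starts a looping timer that moves the handle target to the character's Scene component.
; DontTraction releases the handle and clears that timer; the event graph has no active logic.
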(event EventBeginPlay)

(event Collision|EventActorBeginOverlap
  (params (OtherActor :type Actor%20Object%20Reference)))

(event EventTick
  (params (DeltaSeconds :type Float%20%28single-precision%29)))

(fn ConstructionScript)

(fn AddForce
  (params (Dir :type Vector))
  (Physics|AddImpulse (Variables|Default|GetCube) (* Dir (Variables|Default|GetPower)) "None" true))

(fn Traction
  (bind _cube (Variables|Default|GetCube))
  (Variables|Default|SetLoc (Transformation|GetActorLocation self))
  (bind _returnvalue (Actor|GetActorOfClass "/Game/FirstPerson/Blueprints/BP_FirstPersonCharacter.BP_FirstPersonCharacter_C"))
  (Class|PhysicsHandleComponent|GrabComponentatLocation (Variables|/Game/FirstPerson/Blueprints/BP_FirstPersonCharacter.BP_FirstPersonCharacter_C|GetPhysicsHandle _returnvalue) _cube "None" (Transformation|GetWorldLocation _cube))
  (Physics|SetSimulatePhysics (Variables|Default|GetCube) true)
  (Utilities|Time|SetTimerbyFunctionName 0 "ChangeHandLoc" 0.1 true))

(fn ChangeHandLoc
  (bind _returnvalue (Actor|GetActorOfClass "/Game/FirstPerson/Blueprints/BP_FirstPersonCharacter.BP_FirstPersonCharacter_C"))
  (Physics|Components|PhysicsHandle|SetTargetLocation (Variables|/Game/FirstPerson/Blueprints/BP_FirstPersonCharacter.BP_FirstPersonCharacter_C|GetPhysicsHandle _returnvalue) (Transformation|GetWorldLocation (Variables|/Game/FirstPerson/Blueprints/BP_FirstPersonCharacter.BP_FirstPersonCharacter_C|GetScene _returnvalue))))

(fn DontTraction
  (bind _returnvalue (Actor|GetActorOfClass "/Game/FirstPerson/Blueprints/BP_FirstPersonCharacter.BP_FirstPersonCharacter_C"))
  (Physics|Components|PhysicsHandle|ReleaseComponent (Variables|/Game/FirstPerson/Blueprints/BP_FirstPersonCharacter.BP_FirstPersonCharacter_C|GetPhysicsHandle _returnvalue))
  (Utilities|Time|ClearTimerbyFunctionName 0 "ChangeHandLoc"))