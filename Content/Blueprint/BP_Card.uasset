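; BP_Card is a card pickup that spins continuously in the world through a local rotation applied every Tick.
; EEvent copies the card's First and Second flags onto BP_FirstPersonCharacter's FirstCard and SecondCard, overwriting both values.
; Each true flag also sends its own text to the character's TalkWidget, then the actor destroys itself.
; The rotation step is fixed per frame, so spin speed depends on frame rate.
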(event EventBeginPlay
  (|CallParentFunction) ; This node is disabled and will not be called.\nDrag off pins to build functionality.
)

(event Collision|EventActorBeginOverlap
  (params (OtherActor :type Actor%20Object%20Reference))
  (|CallParentFunction OtherActor) ; This node is disabled and will not be called.\nDrag off pins to build functionality.
)

(event EventTick
  (params (DeltaSeconds :type Float%20%28single-precision%29))
  (|CallParentFunction DeltaSeconds)
  (Transformation|AddLocalRotation (Variables|Default|GetScene) "0.000000,5.000000,0.000000" false false))

(event EventEEvent
  (bind _first (Variables|Default|GetFirst))
  (bind _second (Variables|Default|GetSecond))
  (bind _returnvalue (Actor|GetActorOfClass "/Game/FirstPerson/Blueprints/BP_FirstPersonCharacter.BP_FirstPersonCharacter_C"))
  (Variables|/Game/FirstPerson/Blueprints/BP_FirstPersonCharacter.BP_FirstPersonCharacter_C|SetFirstCard _returnvalue _first)
  (Variables|/Game/FirstPerson/Blueprints/BP_FirstPersonCharacter.BP_FirstPersonCharacter_C|SetSecondCard _returnvalue _second)
  (if _first
    (bind _returnvalue_2 (Actor|GetActorOfClass "/Game/FirstPerson/Blueprints/BP_FirstPersonCharacter.BP_FirstPersonCharacter_C"))
    (Default|AddText (Variables|/Game/FirstPerson/Blueprints/BP_FirstPersonCharacter.BP_FirstPersonCharacter_C|GetTalkWidget _returnvalue_2) (Variables|Default|GetText%20Map_0)))
  (if _second
    (bind _returnvalue_3 (Actor|GetActorOfClass "/Game/FirstPerson/Blueprints/BP_FirstPersonCharacter.BP_FirstPersonCharacter_C"))
    (Default|AddText (Variables|/Game/FirstPerson/Blueprints/BP_FirstPersonCharacter.BP_FirstPersonCharacter_C|GetTalkWidget _returnvalue_3) (Variables|Default|GetText%20Map)))
  (Actor|DestroyActor))

(fn ConstructionScript
  (|CallParentFunction))