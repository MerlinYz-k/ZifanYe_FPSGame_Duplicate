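; BP_Computer is an interactable terminal that checks whether the first-person character holds the matching keycard, selected by its First or Second flag.
; The first card shows dialogue, updates flagged mechanical batteries and auto doors, and turns LightGreen meshes green.
; The second card attaches the computer to the elevator and sends it up.
; A missing card triggers an alarm and temporary warning widget, with IsCanPress blocking repeat presses meanwhile.
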(event EventBeginPlay
  (|CallParentFunction) ; This node is disabled and will not be called.\nDrag off pins to build functionality.
)

(event Collision|EventActorBeginOverlap
  (params (OtherActor :type Actor%20Object%20Reference))
  (|CallParentFunction OtherActor) ; This node is disabled and will not be called.\nDrag off pins to build functionality.
)

(event EventTick
  (params (DeltaSeconds :type Float%20%28single-precision%29))
  (|CallParentFunction DeltaSeconds) ; This node is disabled and will not be called.\nDrag off pins to build functionality.
)

(event EventEEvent
  (if (not (Variables|Default|GetIsCanPress?))
    (Variables|Default|SetIsCanPress? true)
    (bind _returnvalue (Actor|GetActorOfClass "/Game/FirstPerson/Blueprints/BP_FirstPersonCharacter.BP_FirstPersonCharacter_C"))
    (if (Variables|Default|GetFirst)
      (if (Variables|/Game/FirstPerson/Blueprints/BP_FirstPersonCharacter.BP_FirstPersonCharacter_C|GetFirstCard _returnvalue)
        (Audio|PlaySound2D "/Game/sound/stop.stop" 1.0 1.0 0.0 0 0)
        (bind _returnvalue_2 (Actor|GetActorOfClass "/Game/FirstPerson/Blueprints/BP_FirstPersonCharacter.BP_FirstPersonCharacter_C"))
        (Default|AddText (Variables|/Game/FirstPerson/Blueprints/BP_FirstPersonCharacter.BP_FirstPersonCharacter_C|GetTalkWidget _returnvalue_2) (Variables|Default|GetText%20Map))
        (bind _outactors (Actor|GetAllActorsOfClass "/Game/Blueprint/BP_MechanicalBattery.BP_MechanicalBattery_C"))
        (for _array_element _outactors
          (if (Variables|/Game/Blueprint/BP_MechanicalBattery.BP_MechanicalBattery_C|GetFirst _array_element)
            (Default|Close _array_element)
            (Default|ChangeColor _array_element)))
        (bind _outactors_2 (Actor|GetAllActorsOfClass "/Game/Blueprint/BP_AutoDoor.BP_AutoDoor_C"))
        (for _array_element_2 _outactors_2
          (if (Variables|/Game/Blueprint/BP_AutoDoor.BP_AutoDoor_C|GetFirst _array_element_2)
            (Default|Reverse _array_element_2)))
        (bind _outactors_3 (Actor|GetAllActorsOfClass "/Script/Engine.StaticMeshActor"))
        (for _array_element_3 _outactors_3
          (if (Utilities|Enum|Equal(Enum) (Utilities|GetDisplayName _array_element_3) "LightGreen")
            (Rendering|Material|SetMaterial (Variables|/Script/Engine.StaticMeshActor|GetStaticMeshComponent _array_element_3) 0 "/Game/GreenBasicShapeMaterial.GreenBasicShapeMaterial")
            (Variables|Default|SetFirst false)))
        (else
          (Audio|PlaySound2D "/Game/sound/可商用-错误_99-警报音效_爱给网_aigei_com.可商用-错误_99-警报音效_爱给网_aigei_com" 1.0 1.0 0.0 0 0)
          (bind _returnvalue_3 (UserInterface|CreateWidget "/Game/Widget/WB_Warn.WB_Warn_C"))
          (UserInterface|Viewport|AddtoViewport _returnvalue_3 0)
          (Utilities|FlowControl|Delay 4.0)
          (Widget|RemovefromParent _returnvalue_3)
          (Variables|Default|SetIsCanPress? false)))
      (elif (Variables|Default|GetSecond)
        (if (Variables|/Game/FirstPerson/Blueprints/BP_FirstPersonCharacter.BP_FirstPersonCharacter_C|GetSecondCard _returnvalue)
          (Audio|PlaySound2D "/Game/sound/成功提示音__9__爱给网_aigei_com.成功提示音__9__爱给网_aigei_com" 1.0 1.0 0.0 0 0)
          (bind _returnvalue_4 (Actor|GetActorOfClass "/Game/Blueprint/BP_Elevator.BP_Elevator_C"))
          (Transformation|AttachActorToActor self _returnvalue_4 "None" "KeepWorld" "KeepWorld" "KeepWorld" true)
          (Default|UpLoc _returnvalue_4)
          (Variables|Default|SetSecond false)
          (else
            (Audio|PlaySound2D "/Game/sound/可商用-错误_99-警报音效_爱给网_aigei_com.可商用-错误_99-警报音效_爱给网_aigei_com" 1.0 1.0 0.0 0 0)
            (bind _returnvalue_5 (UserInterface|CreateWidget "/Game/Widget/WB_Warn.WB_Warn_C"))
            (UserInterface|Viewport|AddtoViewport _returnvalue_5 0)
            (Utilities|FlowControl|Delay 4.0)
            (Widget|RemovefromParent _returnvalue_5)
            (Variables|Default|SetIsCanPress? false)))))))

(fn ConstructionScript
  (|CallParentFunction))