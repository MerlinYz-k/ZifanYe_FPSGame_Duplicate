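; BP_Door is a door actor opened by its EEvent custom event.
; Each call plays button-press and door-open sounds, then turns the spotlight and Cube10 green as an open indicator.
; An IsOver flag lets the slide run only once: a timeline lerps Cube0 from its starting relative location by subtracting AddLocation.
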(event EventBeginPlay)

(event Collision|EventActorBeginOverlap
  (params (OtherActor :type Actor%20Object%20Reference)))

(event EventTick
  (params (DeltaSeconds :type Float%20%28single-precision%29)))

(event EventEEvent
  (bind _spotlight (Variables|Default|GetSpotLight))
  (Audio|PlaySound2D "/Game/sound/按压按钮.按压按钮" 1.0 1.0 0.0 0 0)
  (Audio|PlaySound2D "/Game/sound/开门.开门" 1.0 1.0 0.0 0 0)
  (Rendering|Components|Light|SetLightColor _spotlight "(R=0.350078,G=1.000000,B=0.000000,A=1.000000)" true)
  (Rendering|Components|Light|SetIntensity _spotlight 5e+02)
  (Rendering|Material|SetMaterial (Variables|Default|GetCube1_0) 0 "/Game/GreenBasicShapeMaterial.GreenBasicShapeMaterial")
  (if (not (Variables|Default|GetIsOver?))
    (Variables|Default|SetIsOver? true)
    (Variables|Default|SetRelative%20Location (Variables|/Script/Engine.SceneComponent|GetRelativeLocation (Variables|Default|GetCube_0)))
    (bind _newtrack_0 (Timeline|Timeline_3 PlayFromStart)
      (:Update
        (Transformation|SetRelativeLocation (Variables|Default|GetCube_0) (Math|Vector|Lerp(Vector) (Variables|Default|GetRelative%20Location) (- (Variables|Default|GetRelative%20Location) (Variables|Default|GetAddLocation)) _newtrack_0) false false)))))

(fn ConstructionScript)