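; Elevator actor that carries the player along a scripted one-way ride, with two moving cubes apparently acting as doors.
; The player overlapping CubeBox slides Cube via a timeline; the UpLoc event reverses it, stops Niagara, then animates the actor's height with sound cues.
; On arrival it relocates Cube1Box and slides Cube1 open.
; Overlapping Cube1Box returns Cube1, adds text to the player's TalkWidget and starts the WB_OverTime timer widget.
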(event OnComponentBeginOverlap(CubeBox)
  (params (OverlappedComponent :type Primitive%20Component%20Object%20Reference) (OtherActor :type Actor%20Object%20Reference) (OtherComp :type Primitive%20Component%20Object%20Reference) (OtherBodyIndex :type Integer) (bFromSweep :type Boolean) (SweepResult :type Hit%20Result%20Structure%20%28by%20ref%29))
  (Utilities|Casting|CastToBP_FirstPersonCharacter OtherActor)
  (Variables|Default|SetNewVar (Transformation|GetWorldLocation (Variables|Default|GetCube)))
  (bind _newtrack_0 (Timeline|Timeline PlayFromStart)
    (:Update
      (Transformation|SetWorldLocation (Variables|Default|GetCube) (Math|Vector|Lerp(Vector) (Variables|Default|GetNewVar) (Variables|Default|GetCubeLoc) _newtrack_0) false false))))

(event OnComponentBeginOverlap(Cube1Box)
  (params (OverlappedComponent :type Primitive%20Component%20Object%20Reference) (OtherActor :type Actor%20Object%20Reference) (OtherComp :type Primitive%20Component%20Object%20Reference) (OtherBodyIndex :type Integer) (bFromSweep :type Boolean) (SweepResult :type Hit%20Result%20Structure%20%28by%20ref%29))
  (Utilities|Casting|CastToBP_FirstPersonCharacter OtherActor)
  (Utilities|FlowControl|Sequence
    (:then_0
      (bind _newtrack_0 (Timeline|Timeline_3 ReverseFromEnd)
        (:Update
          (Transformation|SetWorldLocation (Variables|Default|GetCube1) (Math|Vector|Lerp(Vector) (Variables|Default|Getloc) (Transformation|GetWorldLocation (Variables|Default|GetCube1)) _newtrack_0) false false))))
    (:then_1
      (bind _returnvalue (Actor|GetActorOfClass "/Game/FirstPerson/Blueprints/BP_FirstPersonCharacter.BP_FirstPersonCharacter_C"))
      (Default|AddText (Variables|/Game/FirstPerson/Blueprints/BP_FirstPersonCharacter.BP_FirstPersonCharacter_C|GetTalkWidget _returnvalue) (Variables|Default|GetText%20Map)))
    (:then_2
      (bind _returnvalue_2 (UserInterface|CreateWidget "/Game/Widget/WB_OverTime.WB_OverTime_C"))
      (Default|TimeStart _returnvalue_2)
      (UserInterface|Viewport|AddtoViewport _returnvalue_2 0))))

(event Custom|UpLoc
  (Audio|PlaySound2D "/Game/sound/123.123" 1.0 1.0 0.0 0 0)
  (bind _newtrack_0 (Timeline|Timeline_0 ReverseFromEnd)
    (:Update
      (Transformation|SetWorldLocation (Variables|Default|GetCube) (Math|Vector|Lerp(Vector) (Variables|Default|GetNewVar) (Variables|Default|GetCubeLoc) _newtrack_0) false false))
    (:Finished
      (Components|Activation|SetActive (Variables|Default|GetNiagara) false false)
      (Audio|PlaySound2D "/Game/sound/运行.运行" 1.0 1.0 0.0 0 0)
      (bind _newtrack_0_2 (Timeline|Timeline_1 PlayFromStart)
        (:Update
          (Transformation|SetActorLocation (Math|Vector|MakeVector -10408.832333 -3418.943618 _newtrack_0_2) false false))
        (:Finished
          (Transformation|SetWorldLocation (Variables|Default|GetCube1Box) "-11302.948510,-2696.729798,5054.176830" false false)
          (Variables|Default|Setloc (Transformation|GetWorldLocation (Variables|Default|GetCube1)))
          (Audio|PlaySound2D "/Game/sound/电梯到达.电梯到达" 1.0 1.0 0.0 0 0)
          (bind _newtrack_0_3 (Timeline|Timeline_2 PlayFromStart)
            (:Update
              (Transformation|SetWorldLocation (Variables|Default|GetCube1) (Math|Vector|Lerp(Vector) (Transformation|GetWorldLocation (Variables|Default|GetCube1)) (Variables|Default|GetCube1Loc) _newtrack_0_3) false false))))))))

(event EventBeginPlay
  (Variables|Default|Setloc (Transformation|GetWorldLocation (Variables|Default|GetCube1))))

(event Collision|EventActorBeginOverlap
  (params (OtherActor :type Actor%20Object%20Reference)))

(event EventTick
  (params (DeltaSeconds :type Float%20%28single-precision%29)))

(fn ConstructionScript)