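; Elevator platform Blueprint that shuttles Cube0 between FirstLocation and LastLoc each time EEvent fires.
; IsOver locks out triggers during travel, while IsReverse flips on completion to select the next direction.
; Each trip plays door-open and button-press sounds, colors Cube0 and Cube10 green outbound or red returning, and lerps position through a per-direction Timeline.
; Debug strings print when each trip finishes.
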(event EventEEvent
  (if (not (Variables|Default|GetIsOver?))
    (Audio|PlaySound2D "/Game/sound/开门.开门" 1.0 1.0 0.0 0 0)
    (Audio|PlaySound2D "/Game/sound/按压按钮.按压按钮" 1.0 1.0 0.0 0 0)
    (if (Variables|Default|GetIsReverse?)
      (Variables|Default|SetIsOver? true)
      (Rendering|Material|SetMaterial (Variables|Default|GetCube_0) 0 "/Game/RedBasicShapeMaterial1.RedBasicShapeMaterial1")
      (Rendering|Material|SetMaterial (Variables|Default|GetCube1_0) 0 "/Game/RedBasicShapeMaterial1.RedBasicShapeMaterial1")
      (bind _newtrack_0 (Timeline|Timeline PlayFromStart)
        (:Update
          (Transformation|SetWorldLocation (Variables|Default|GetCube_0) (Math|Vector|Lerp(Vector) (Variables|Default|GetLastLoc) (Variables|Default|GetFirstLocation) _newtrack_0) false false))
        (:Finished
          (Development|PrintString (Utilities|String|ToString(Vector) "0, 0, 0") true true "(R=0.451393,G=0.015590,B=1.000000,A=1.000000)")
          (Variables|Default|SetIsOver? false)
          (Variables|Default|SetIsReverse? false)))
      (else
        (Variables|Default|SetIsOver? true)
        (Rendering|Material|SetMaterial (Variables|Default|GetCube_0) 0 "/Game/GreenBasicShapeMaterial.GreenBasicShapeMaterial")
        (Rendering|Material|SetMaterial (Variables|Default|GetCube1_0) 0 "/Game/GreenBasicShapeMaterial.GreenBasicShapeMaterial")
        (bind _newtrack_0_2 (Timeline|Timeline_3 PlayFromStart)
          (:Update
            (Transformation|SetWorldLocation (Variables|Default|GetCube_0) (Math|Vector|Lerp(Vector) (Variables|Default|GetFirstLocation) (Variables|Default|GetLastLoc) _newtrack_0_2) false false))
          (:Finished
            (Development|PrintString "Hello" true true "(R=0.978515,G=1.000000,B=0.106585,A=1.000000)")
            (Variables|Default|SetIsOver? false)
            (Variables|Default|SetIsReverse? true)))))))

(fn ConstructionScript)