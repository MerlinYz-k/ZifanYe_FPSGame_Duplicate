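; BP_Explosion is an explosion effect Blueprint that plays randomized blasts repeatedly once StartExplosion is called.
; A looping timer fires RandomExplosion, where a random Delay staggers each blast and ignores timer ticks that arrive while it is pending.
; Each blast shakes the first player's camera, swaps a random system from an array onto its Niagara component, and plays a random non-spatial 2D sound.
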(event Custom|StartExplosion
  (Utilities|Time|SetTimerbyEvent (delegate Custom|RandomExplosion) 2.0 true))

(event Custom|RandomExplosion
  (Utilities|FlowControl|Delay (Math|Random|RandomFloatinRange 0.0 3.0))
  (Game|Feedback|ClientStartCameraShake (Game|GetPlayerController 0) "/Game/Explosions_Niagara/Blueprint/BP_Camera_Shake01.BP_Camera_Shake01_C" 5e+01 "World" "0, 0, 0")
  (Class|NiagaraComponent|SetAsset (Variables|Default|GetNiagara) (Utilities|Array|Get(acopy) (Variables|Default|GetArrary_Niagara) (Math|Conversions|ToInteger(Byte) (Class|KismetMathLibrary|RandomInteger64inRange 0 9))) true)
  (Audio|PlaySound2D (Utilities|Array|Get(acopy) (Variables|Default|GetSound) (Math|Random|RandomIntegerinRange 0 1)) 1.0 1.0 0.0 0 0))

(event EventBeginPlay)

(event Collision|EventActorBeginOverlap
  (params (OtherActor :type Actor%20Object%20Reference)))

(event EventTick
  (params (DeltaSeconds :type Float%20%28single-precision%29)))

(fn ConstructionScript)