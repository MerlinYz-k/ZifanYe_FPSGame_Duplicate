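; BP_Information is a spinning pickup actor that shows an information screen when the first-person character touches it.
; Its static mesh rotates by a fixed step each tick.
; On capsule overlap it hides the character's TalkWidget and creates a WB_Information widget filled with its Text0 variable.
; It then shows the mouse cursor, pauses the game and destroys itself, so it triggers only once.
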(event OnComponentBeginOverlap(Capsule)
  (params (OverlappedComponent :type Primitive%20Component%20Object%20Reference) (OtherActor :type Actor%20Object%20Reference) (OtherComp :type Primitive%20Component%20Object%20Reference) (OtherBodyIndex :type Integer) (bFromSweep :type Boolean) (SweepResult :type Hit%20Result%20Structure%20%28by%20ref%29))
  (bind _asbp_first_person_character (Utilities|Casting|CastToBP_FirstPersonCharacter OtherActor))
  (Widget|SetVisibility (Variables|/Game/FirstPerson/Blueprints/BP_FirstPersonCharacter.BP_FirstPersonCharacter_C|GetTalkWidget _asbp_first_person_character) "Hidden")
  (bind _returnvalue (UserInterface|CreateWidget "/Game/Widget/WB_Information.WB_Information_C"))
  (Variables|/Game/Widget/WB_Information.WB_Information_C|SetText _returnvalue (Variables|Default|GetText_0))
  (UserInterface|Viewport|AddtoViewport _returnvalue 0)
  (Variables|/Script/Engine.PlayerController|SetbShowMouseCursor (Game|GetPlayerController 0) true)
  (Game|SetGamePaused true)
  (Actor|DestroyActor))

(event EventBeginPlay)

(event Collision|EventActorBeginOverlap
  (params (OtherActor :type Actor%20Object%20Reference)))

(event EventTick
  (params (DeltaSeconds :type Float%20%28single-precision%29))
  (Transformation|AddLocalRotation (Variables|Default|GetStaticMesh) "0.000000,5.000000,0.000000" false false))

(fn ConstructionScript)