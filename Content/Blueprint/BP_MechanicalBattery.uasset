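; BP_MechanicalBattery is a turret that tracks and shoots the first-person player inside its trigger box.
; Box overlap starts looping timers that turn the mesh toward the player camera and fire BP_Projectile_17 at the capsule, clearing them on exit.
; Damage destroys it at zero health, and a turret flagged Last also calls LastMove on the last BP_AutoDoor.
; Close disables the trigger, and ChangeColor swaps in a green material.
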(event OnComponentBeginOverlap(Box)
  (params (OverlappedComponent :type Primitive%20Component%20Object%20Reference) (OtherActor :type Actor%20Object%20Reference) (OtherComp :type Primitive%20Component%20Object%20Reference) (OtherBodyIndex :type Integer) (bFromSweep :type Boolean) (SweepResult :type Hit%20Result%20Structure%20%28by%20ref%29))
  (bind _asbp_first_person_character (Utilities|Casting|CastToBP_FirstPersonCharacter OtherActor))
  (Variables|Default|SetAs%20BP%20First%20Person%20Character _asbp_first_person_character)
  (bind _returnvalue (Utilities|Time|SetTimerbyEvent (delegate Custom|ShootPlayer) (Math|Conversions|ToFloat(Integer) (Variables|Default|GetShootTime)) true))
  (bind _returnvalue_2 (Utilities|Time|SetTimerbyEvent (delegate Custom|BatteryRotator) 0.01 true)))

(event OnComponentEndOverlap(Box)
  (params (OverlappedComponent :type Primitive%20Component%20Object%20Reference) (OtherActor :type Actor%20Object%20Reference) (OtherComp :type Primitive%20Component%20Object%20Reference) (OtherBodyIndex :type Integer))
  (Utilities|Casting|CastToBP_FirstPersonCharacter OtherActor)
  (Variables|Default|SetAs%20BP%20First%20Person%20Character 0)
  (Utilities|Time|ClearandInvalidateTimerbyHandle (stale OnComponentBeginOverlap(Box) _returnvalue))
  (Utilities|Time|ClearandInvalidateTimerbyHandle (stale OnComponentBeginOverlap(Box) _returnvalue_2)))

(event Custom|ShootPlayer
  (bind _scene (Variables|Default|GetScene))
  (bind _returnvalue (Transformation|GetWorldLocation _scene))
  (bind _returnvalue_2 (Game|SpawnActorfromClass "/Game/ProjectilesVol1/Blueprints/BP_Projectile_17.BP_Projectile_17_C" (Math|Transform|MakeTransform _returnvalue (Math|Rotator|FindLookatRotation _returnvalue (Transformation|GetWorldLocation (Variables|/Script/Engine.Character|GetCapsuleComponent (Variables|Default|GetAs%20BP%20First%20Person%20Character))))) "Undefined" "MultiplyWithRoot" 0 0))
  (Audio|PlaySound2D "/Game/sound/激光射击02_爱给网_aigei_com.激光射击02_爱给网_aigei_com" 1.0 1.0 0.0 0 0)
  (Variables|/Game/ProjectilesVol1/Blueprints/BP_Projectile.BP_Projectile_C|SetParent _returnvalue_2 self)
  (Variables|/Script/Engine.ProjectileMovementComponent|SetInitialSpeed (Actor|GetComponentbyClass _returnvalue_2 "/Script/Engine.ProjectileMovementComponent") (Variables|Default|GetInitial%20Speed))
  (Variables|/Game/ProjectilesVol1/Blueprints/BP_Projectile.BP_Projectile_C|SetNum _returnvalue_2 5))

(event Custom|BatteryRotator
  (Transformation|SetWorldRotation (Variables|Default|GetStaticMesh) (Math|Rotator|FindLookatRotation (Transformation|GetWorldLocation (Variables|Default|GetScene)) (Transformation|GetWorldLocation (Variables|/Game/FirstPerson/Blueprints/BP_FirstPersonCharacter.BP_FirstPersonCharacter_C|GetFirstPersonCamera (Variables|Default|GetAs%20BP%20First%20Person%20Character)))) false false))

(event Custom|ChangeColor
  (Rendering|Material|SetMaterial (Variables|Default|GetSkeletalMesh) 1 "/Game/GreenBasicShapeMaterial.GreenBasicShapeMaterial")
  (Rendering|Material|SetMaterial (Variables|Default|GetStaticMesh) 1 "/Game/GreenBasicShapeMaterial.GreenBasicShapeMaterial"))

(event EventBeginPlay)

(event Collision|EventActorBeginOverlap
  (params (OtherActor :type Actor%20Object%20Reference)))

(event EventTick
  (params (DeltaSeconds :type Float%20%28single-precision%29)))

(fn ConstructionScript)

(fn Damage
  (params (DamageNum :type Integer))
  (bind _output_get (Variables|Default|SetHealthy (- (Variables|Default|GetHealthy) DamageNum)))
  (if (<= _output_get 0)
    (if (Variables|Default|GetLast)
      (bind _outactors (Actor|GetAllActorsOfClass "/Game/Blueprint/BP_AutoDoor.BP_AutoDoor_C"))
      (for _array_element _outactors
        (if (Variables|/Game/Blueprint/BP_AutoDoor.BP_AutoDoor_C|GetIsLast? _array_element)
          (Default|LastMove _array_element))))
    (Actor|DestroyActor)))

(fn Close
  (Collision|SetCollisionEnabled (Variables|Default|GetBox) "NoCollision"))