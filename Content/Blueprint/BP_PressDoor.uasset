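; Pressure-plate door that opens while a BP_Box or the first-person character stands on it and closes on exit.
; Box overlaps play sounds, switch the Cube1 plate between green and red, and toggle the SpotLight.
; Separate open and close timelines lerp Door between its BeginPlay location and that minus ChangeVec, while others nudge Cube1 incrementally down or up.
; Occupants are not counted, so any valid exit triggers closing.
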(event OnComponentBeginOverlap(Box)
  (params (OverlappedComponent :type Primitive%20Component%20Object%20Reference) (OtherActor :type Actor%20Object%20Reference) (OtherComp :type Primitive%20Component%20Object%20Reference) (OtherBodyIndex :type Integer) (bFromSweep :type Boolean) (SweepResult :type Hit%20Result%20Structure%20%28by%20ref%29))
  (bind _loc (Variables|Default|GetLoc))
  (bind _cube1 (Variables|Default|GetCube1))
  (bind _returnvalue (Transformation|GetWorldLocation _cube1))
  (Utilities|Casting|CastToBP_Box OtherActor
    (:then
      _)
    (:CastFailed
      (Utilities|Casting|CastToBP_FirstPersonCharacter OtherActor)))
  (Audio|PlaySound2D "/Game/sound/开门.开门" 1.0 1.0 0.0 0 0)
  (Audio|PlaySound2D "/Game/sound/按压按钮.按压按钮" 1.0 1.0 0.0 0 0)
  (Rendering|Material|SetMaterial (Variables|Default|GetCube1) 0 "/Game/GreenBasicShapeMaterial.GreenBasicShapeMaterial")
  (Rendering|Components|Light|SetIntensity (Variables|Default|GetSpotLight) 5e+02)
  (Utilities|FlowControl|Sequence
    (:then_0
      (bind _newtrack_0 (Timeline|Timeline PlayFromStart)
        (:Update
          (Transformation|SetWorldLocation (Variables|Default|GetDoor) (Math|Vector|Lerp(Vector) _loc (- _loc (Variables|Default|GetChangeVec)) _newtrack_0) false false))))
    (:then_1
      (bind _newtrack_0_2 (Timeline|Timeline_1 PlayFromStart)
        (:Update
          (Transformation|SetWorldLocation _cube1 (Math|Vector|Lerp(Vector) _returnvalue (- _returnvalue "0.000000,0.000000,0.100000") _newtrack_0_2) false false))))))

(event OnComponentEndOverlap(Box)
  (params (OverlappedComponent :type Primitive%20Component%20Object%20Reference) (OtherActor :type Actor%20Object%20Reference) (OtherComp :type Primitive%20Component%20Object%20Reference) (OtherBodyIndex :type Integer))
  (bind _cube1 (Variables|Default|GetCube1))
  (bind _loc (Variables|Default|GetLoc))
  (bind _returnvalue (Transformation|GetWorldLocation _cube1))
  (Utilities|Casting|CastToBP_Box OtherActor
    (:then
      _)
    (:CastFailed
      (Utilities|Casting|CastToBP_FirstPersonCharacter OtherActor)))
  (Audio|PlaySound2D "/Game/sound/开门.开门" 1.0 1.0 0.0 0 0)
  (Audio|PlaySound2D "/Game/sound/按压按钮.按压按钮" 1.0 1.0 0.0 0 0)
  (Rendering|Material|SetMaterial (Variables|Default|GetCube1) 0 "/Game/RedBasicShapeMaterial1.RedBasicShapeMaterial1")
  (Rendering|Components|Light|SetIntensity (Variables|Default|GetSpotLight) 0.0)
  (Utilities|FlowControl|Sequence
    (:then_0
      (bind _newtrack_0 (Timeline|Timeline_0 PlayFromStart)
        (:Update
          (Transformation|SetWorldLocation (Variables|Default|GetDoor) (Math|Vector|Lerp(Vector) (- _loc (Variables|Default|GetChangeVec)) _loc _newtrack_0) false false))))
    (:then_1
      (bind _newtrack_0_2 (Timeline|Timeline_2 PlayFromStart)
        (:Update
          (Transformation|SetWorldLocation _cube1 (Math|Vector|Lerp(Vector) _returnvalue (+ _returnvalue "0.000000,0.000000,0.100000") _newtrack_0_2) false false))))))

(event EventBeginPlay
  (Variables|Default|SetLoc (Transformation|GetWorldLocation (Variables|Default|GetDoor))))

(event Collision|EventActorBeginOverlap
  (params (OtherActor :type Actor%20Object%20Reference)))

(event EventTick
  (params (DeltaSeconds :type Float%20%28single-precision%29)))

(fn ConstructionScript)