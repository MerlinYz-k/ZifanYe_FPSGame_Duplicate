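; BP_PressE is an interactable actor with a trigger Box that marks when the first-person player is in range.
; It finds BP_FirstPersonCharacter on BeginPlay.
; Box overlap shows or hides the text on the player's SightBead widget and sets or clears itself as the player's PressEObject.
; E_Event is an empty hook for the interaction, with no behavior in this Blueprint.
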(event OnComponentBeginOverlap(Box)
  (params (OverlappedComponent :type Primitive%20Component%20Object%20Reference) (OtherActor :type Actor%20Object%20Reference) (OtherComp :type Primitive%20Component%20Object%20Reference) (OtherBodyIndex :type Integer) (bFromSweep :type Boolean) (SweepResult :type Hit%20Result%20Structure%20%28by%20ref%29))
  (bind _player (Variables|Default|GetPlayer))
  (Utilities|Casting|CastToBP_FirstPersonCharacter OtherActor)
  (Widget|SetVisibility (Variables|/Game/Widget/WB_SightBead.WB_SightBead_C|GetTextBlock_0 (Variables|/Game/FirstPerson/Blueprints/BP_FirstPersonCharacter.BP_FirstPersonCharacter_C|GetSightBead _player)) "Visible")
  (Variables|/Game/FirstPerson/Blueprints/BP_FirstPersonCharacter.BP_FirstPersonCharacter_C|SetPressEObject _player self))

(event OnComponentEndOverlap(Box)
  (params (OverlappedComponent :type Primitive%20Component%20Object%20Reference) (OtherActor :type Actor%20Object%20Reference) (OtherComp :type Primitive%20Component%20Object%20Reference) (OtherBodyIndex :type Integer))
  (bind _player (Variables|Default|GetPlayer))
  (Utilities|Casting|CastToBP_FirstPersonCharacter OtherActor)
  (Widget|SetVisibility (Variables|/Game/Widget/WB_SightBead.WB_SightBead_C|GetTextBlock_0 (Variables|/Game/FirstPerson/Blueprints/BP_FirstPersonCharacter.BP_FirstPersonCharacter_C|GetSightBead _player)) "Hidden")
  (Variables|/Game/FirstPerson/Blueprints/BP_FirstPersonCharacter.BP_FirstPersonCharacter_C|SetPressEObject _player 0))

(event Custom|E_Event)

(event EventBeginPlay
  (bind _returnvalue (Actor|GetActorOfClass "/Game/FirstPerson/Blueprints/BP_FirstPersonCharacter.BP_FirstPersonCharacter_C"))
  (Variables|Default|SetPlayer _returnvalue))

(event Collision|EventActorBeginOverlap
  (params (OtherActor :type Actor%20Object%20Reference)))

(event EventTick
  (params (DeltaSeconds :type Float%20%28single-precision%29)))

(fn ConstructionScript)