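; BP_Slope is a level actor with a button-like, one-shot moving Plane triggered by EEvent.
; Each trigger plays door-open and button-press sounds and turns Cube10 green.
; Only the first stores the Plane's world location and runs a timeline lerping it to AddLocation2, used as an absolute position rather than an offset.
; An opposite-offset move for Plane1 is left disconnected.
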(event Collision|EventActorBeginOverlap
  (params (OtherActor :type Actor%20Object%20Reference)))

(event EventTick
  (params (DeltaSeconds :type Float%20%28single-precision%29)))

(event EventEEvent
  (Audio|PlaySound2D "/Game/sound/开门.开门" 1.0 1.0 0.0 0 0)
  (Audio|PlaySound2D "/Game/sound/按压按钮.按压按钮" 1.0 1.0 0.0 0 0)
  (Rendering|Material|SetMaterial (Variables|Default|GetCube1_0) 0 "/Game/GreenBasicShapeMaterial.GreenBasicShapeMaterial")
  (if (not (Variables|Default|GetIsOver?))
    (bind _output_get (Variables|Default|SetLoc (Transformation|GetWorldLocation (Variables|Default|GetPlane))))
    (Variables|Default|SetIsOver? true)
    (bind _newtrack_0 (Timeline|Timeline_3 PlayFromStart)
      (:Update
        (Transformation|SetWorldLocation (Variables|Default|GetPlane) (Math|Vector|Lerp(Vector) _output_get (Variables|Default|GetAddLocation2) _newtrack_0) false false)))))

(fn ConstructionScript)