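; Projectile actor from the ProjectilesVol1 content that spawns a flash effect on spawn and self-destructs after a fixed lifetime.
; Sphere overlap with a first-person character calls its Heart function and destroys the projectile, provided Parent is valid.
; Hits on anything else spawn an offset impact effect, oriented by the surface normal or actor rotation depending on flags, then switch off the light and destroy the actor after a delay.
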(event OnComponentHit(Sphere)
  (params (HitComponent :type Primitive%20Component%20Object%20Reference) (OtherActor :type Actor%20Object%20Reference) (OtherComp :type Primitive%20Component%20Object%20Reference) (NormalImpulse :type Vector :default "0, 0, 0") (Hit :type Hit%20Result%20Structure%20%28by%20ref%29))
  (bind _returnvalue (Transformation|GetActorRotation))
  (bind (_bblockinghit _binitialoverlap _time _distance _location _impactpoint _normal _impactnormal) (Collision|BreakHitResult Hit))
  (Utilities|Casting|CastToBP_FirstPersonCharacter OtherActor
    (:CastFailed
      (if (Variables|Default|GetUse%20zero%20rotation)
        (Variables|Default|SetRotation _returnvalue)
        (elif (Variables|Default|GetUse%20self%20rotation)
          (Variables|Default|SetRotation _returnvalue)
          (else
            (Variables|Default|SetRotation (Math|Rotator|MakeRotfromX _impactnormal)))))
      (Niagara|SpawnSystematLocation (Variables|Default|GetHit%20effect) (+ _location (* _impactnormal (Variables|Default|GetHit%20offset))) (Variables|Default|GetRotation))
      (Rendering|Components|Light|SetIntensity (Variables|Default|GetPointLight) 0.0)
      (Utilities|FlowControl|Delay (Variables|Default|GetProjectile%20hit%20destroy%20delay))
      (Actor|DestroyActor))))

(event OnComponentBeginOverlap(Sphere)
  (params (OverlappedComponent :type Primitive%20Component%20Object%20Reference) (OtherActor :type Actor%20Object%20Reference) (OtherComp :type Primitive%20Component%20Object%20Reference) (OtherBodyIndex :type Integer) (bFromSweep :type Boolean) (SweepResult :type Hit%20Result%20Structure%20%28by%20ref%29))
  (Utilities|IsValid (Variables|Default|GetParent)
    (:Is%20Valid
      (bind _asbp_first_person_character (Utilities|Casting|CastToBP_FirstPersonCharacter OtherActor))
      (Default|Heart _asbp_first_person_character 10)
      (Actor|DestroyActor))))

(event EventBeginPlay
  (Niagara|SpawnSystematLocation (Variables|Default|GetFlash%20effect) (Transformation|GetActorLocation) (Transformation|GetActorRotation))
  (Utilities|FlowControl|Delay 1e+01)
  (Actor|DestroyActor))

(fn ConstructionScript)